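; BP_Ceiling_Lamps is an interactable ceiling lamp whose point light toggles on and off.
; The Interaction event flips LampPower, and its OnRep function applies the value to the PointLight's visibility.
; The construction script applies the same visibility, so the initial state follows LampPower.
; The health and inventory system getters are empty stubs.
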(event `/Game/VisualSandbox/Blueprints/Interfaces/BPI_Useful.Receive Interaction`
  (params (`Interaction Actor` :type "Actor Object Reference") (`Interaction Instigator` :type "Controller Object Reference"))
  (set `self.Lamp Power` (not (`self.Lamp Power`))))

(fn `Get Health System`
  (returns (`Health Conp` :type "/Game/VisualSandbox/Blueprints/Components/AC_HealthComponent Object Reference"))
  (return null))

(fn `Get Inventory System`
  (returns (`Inventory Comp` :type "/Game/VisualSandbox/Blueprints/Components/AC_InventoryComponent Object Reference"))
  (return null))

(fn `OnRep_Lamp Power`
  (`SceneComponent.SetVisibility` (`self.PointLight`) (`self.Lamp Power`) false))

(fn `UserConstructionScript`
  (`SceneComponent.SetVisibility` (`self.PointLight`) (`self.Lamp Power`) false))