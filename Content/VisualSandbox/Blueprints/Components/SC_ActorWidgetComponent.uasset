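; Widget component that shows an actor-attached widget only when the player pawn is near and, unless x-ray is enabled, in unobstructed view.
; BeginPlay passes the owning actor to the widget via SetupOwnerMessage.
; Each tick compares squared distance directly to VisibleDistance, so that value is in squared units.
; CheckXRay line-traces to the camera on XRayBlockingChannel, ignoring the owner; EnableXRay skips the trace.
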(event `self.ReceiveBeginPlay`
  ; Setup widget owner automatically
  (message `/Game/VisualSandbox/Blueprints/Interfaces/BPI_Useful.Setup Owner` (`self.GetUserWidgetObject`) (`self.GetOwner`)))

(event `self.ReceiveTick`
  (params (DeltaSeconds :type "Float (single-precision)"))
  ; Calculates visible distance and x-ray
  (set `Widget.Visibility` (select `bool` (and (<= (`KismetMathLibrary.Vector_DistanceSquared` (`self.K2_GetComponentLocation`) (`Actor.K2_GetActorLocation` (`GameplayStatics.GetPlayerPawn` 0))) (`self.Visible Distance`)) (`self.Check X-Ray`)) :`false` "Hidden" :`true` "SelfHitTestInvisible" :!type "ESlateVisibility Enum") (`self.GetUserWidgetObject`)))

(fn `Check X-Ray`
  (returns (ReturnValue :type Boolean))
  (if (`self.Enable X-Ray`)
    (return true)
    (else
      (bind _outhit (`KismetSystemLibrary.LineTraceSingle` (`self.K2_GetComponentLocation`) (`Actor.GetActorEyesViewPoint` (`GameplayStatics.GetPlayerCameraManager` 0)) (`self.X-Ray Blocking Channel`) false (`|MakeArray` (`self.GetOwner`))))
      (return (not (`GameplayStatics.BreakHitResult` _outhit))))))