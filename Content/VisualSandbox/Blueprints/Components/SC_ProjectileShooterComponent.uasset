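; Scene component that acts as a weapon muzzle, spawning projectiles along its own rotation or a supplied shoot direction.
; FireProjectile spawns one or more spread projectiles on the authority only, passing damage and instigator, then reports an AI noise event.
; Firing FX, sound and the ShotsFired dispatcher run wherever it is called, regardless of authority.
; Tick runs a forward line trace every frame, drawn as a debug laser when enabled.
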(event `self.ReceiveTick`
  (params (DeltaSeconds :type "Float (single-precision)"))
  (bind _returnvalue (`self.K2_GetComponentLocation`))
  (`KismetSystemLibrary.LineTraceSingle` :`Start` _returnvalue :`End` (`/Game/VisualSandbox/Blueprints/Utility/BP_UsefulFunctions.Get Forward Location` _returnvalue (`self.K2_GetComponentRotation`) 1000000.0) :`TraceChannel` "TraceTypeQuery3" :`DrawDebugType` (select `bool` (`self.Draw Debug Laser`) :`true` "ForOneFrame" :!type "EDrawDebugTrace Enum")))

(fn `Fire Projectile`
  (params (`Shoot Direction` :type "Rotator Structure"))
  (locals (`Desired Shoot Direction` :type "Rotator Structure" :default (struct)))
  (bind _returnvalue (`self.GetOwner`))
  (bind (_deviation_angle_x _deviation_angle_y) (`KismetMathLibrary.BreakVector2D` (`self.Deviation Angle`)))
  (bind _shoot_direction (`local.Shoot Direction`))
  (set `local.Desired Shoot Direction` (`KismetMathLibrary.SelectRotator` _shoot_direction (`self.K2_GetComponentRotation`) (!= _shoot_direction (struct))))
  (`|ExecutionSequence`
    (:`then_0`
      (`/Engine/EditorBlueprintResources/ActorComponentMacros.Switch Has Authority` :!pinned true ; Check server authority
        (:`Authority`
          ;[0.15 0.15 1 0.5] Loopbody to spawn single or multiple shots
          (for _ (range 1 (+ (`KismetMathLibrary.Max` (`self.Number Of Shots`) 1) 1))
            ;[0.15 0.15 1 0.5] Spawn brand new projectile actor
            (`|SpawnActorFromClass` (`self.Projectile Class`) (`KismetMathLibrary.MakeTransform` (`self.K2_GetComponentLocation`) (`/Game/VisualSandbox/Blueprints/Utility/BP_UsefulFunctions.Spread Rotation` (`local.Desired Shoot Direction`) (`KismetMathLibrary.MakeRotator` 0.0 _deviation_angle_x _deviation_angle_y))) "AdjustIfPossibleButDontSpawnIfColliding" "MultiplyWithRoot" _returnvalue (`self.Projectile Damage`) (`Actor.Instigator` _returnvalue)))
          ;[0.15 0.15 1 0.5] Report firing noise event
          (`AISense_Hearing.ReportNoiseEvent` (`self.K2_GetComponentLocation`) (`self.Noise Loudness`) (`self.GetOwner`) (`self.Noise Max Range`) (`self.Noise Event Tag`)))))
    (:`then_1`
      ; Play Firing Sound And Effect
      (`NiagaraFunctionLibrary.SpawnSystemAttached` (`self.Firing FX`) self "None" (0.0 0.0 0.0) (`self.Firing FX Orientation`) "SnapToTarget") ; Spawn muzzle flash effect
      (`GameplayStatics.PlaySoundAtLocation` (`self.Firing Sound`) (`self.K2_GetComponentLocation`) (struct) 1.0 1.0 0.0 null null (`self.GetOwner`) null) ; Play Firing sound at component location
      (`self.Shots Fired`) ; Call shots fired dispatcher event\nthat can used by the owner to notify each shot
    )))