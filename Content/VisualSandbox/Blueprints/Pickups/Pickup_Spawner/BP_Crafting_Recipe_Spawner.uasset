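; Crafting recipe pickup that teaches the recipient a recipe by adding its item class to their inventory component.
; CanPickUp requires a valid class, then uses a condition list to reject already-known recipes or items without crafting ingredients, returning a fail reason.
; PickUp gets the inventory component through an interface message, adds the class uniquely to InitialCraftingRecipes and fires the inventory-updated call.
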(fn `Can Pick Up`
  (returns (ReturnValue :type Boolean) (`Fail Reason` :type String))
  (locals (`Inventory Comp` :type "/Game/VisualSandbox/Blueprints/Components/AC_InventoryComponent Object Reference"))
  (`self.Item Recipe Class`
    (:`then`
      (bind _inventory_comp (message `/Game/VisualSandbox/Blueprints/Interfaces/BPI_Useful.Get Inventory System` (`self.Recipient`)))
      (bind _output_get (set `local.Inventory Comp` _inventory_comp))
      (`/Engine/EditorBlueprintResources/StandardMacros.IsValid` _output_get
        (:`Is Valid`
          (bind (_returnvalue _fail_reason) (`/Game/VisualSandbox/Blueprints/Utility/BP_UsefulFunctions.Check Condition List` (`|MakeArray` (make `/Game/VisualSandbox/Blueprints/Structures/FConditionList` (not (`KismetArrayLibrary.Array_Contains` (`/Game/VisualSandbox/Blueprints/Components/AC_InventoryComponent.Initial Crafting Recipes` (`local.Inventory Comp`)) (`self.Item Recipe Class`))) "It already has this recipe") (make `/Game/VisualSandbox/Blueprints/Structures/FConditionList` (`KismetArrayLibrary.Array_IsNotEmpty` (`.Ingredient for Crafting` (defaults `Object` (`self.Item Recipe Class`)))) "It's not craftable item"))))
          (return _returnvalue _fail_reason))))
    (:`else`
      (return false "Invalid recipe class"))))

(fn `Pick Up`
  (locals (`Recipient Inventory Comp` :type "/Game/VisualSandbox/Blueprints/Components/AC_InventoryComponent Object Reference"))
  (bind _inventory_comp (message `/Game/VisualSandbox/Blueprints/Interfaces/BPI_Useful.Get Inventory System` (`self.Recipient`)))
  (bind _output_get (set `local.Recipient Inventory Comp` _inventory_comp))
  (`KismetArrayLibrary.Array_AddUnique` (`/Game/VisualSandbox/Blueprints/Components/AC_InventoryComponent.Initial Crafting Recipes` _output_get) (`self.Item Recipe Class`))
  (`/Game/VisualSandbox/Blueprints/Components/AC_InventoryComponent.On Inventory Updated` (`local.Recipient Inventory Comp`)))

(fn `UserConstructionScript`
  (`parent.UserConstructionScript`))