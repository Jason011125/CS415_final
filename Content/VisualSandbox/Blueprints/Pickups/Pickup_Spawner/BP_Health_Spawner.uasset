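; BP_Health_Spawner is a health pickup spawner that heals the character who picks it up.
; It overrides Can Pick Up to allow only a BP_MasterCharacter recipient that is alive and below full health.
; Pick Up then adds HealAmount through that character's CharacterHealth.
; The event graph is empty and construction only calls the parent, so this Blueprint defines no spawning logic of its own.
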(fn `Can Pick Up`
  (returns (ReturnValue :type Boolean) (`Fail Reason` :type String))
  (bind _asbp_master_character (cast `/Game/VisualSandbox/Blueprints/Characters/BP_MasterCharacter` (`self.Recipient`)))
  (bind _character_health (`/Game/VisualSandbox/Blueprints/Characters/BP_MasterCharacter.Character Health` _asbp_master_character))
  (return (and (not (`/Game/VisualSandbox/Blueprints/Components/AC_HealthComponent.Health Is Full` _character_health)) (`/Game/VisualSandbox/Blueprints/Components/AC_HealthComponent.Is Alive` _character_health)) ""))

(fn `Pick Up`
  (bind _asbp_master_character (cast `/Game/VisualSandbox/Blueprints/Characters/BP_MasterCharacter` (`self.Recipient`)))
  (`/Game/VisualSandbox/Blueprints/Components/AC_HealthComponent.Add Health` (`/Game/VisualSandbox/Blueprints/Characters/BP_MasterCharacter.Character Health` _asbp_master_character) (`self.Heal Amount`)))

(fn `UserConstructionScript`
  (`parent.UserConstructionScript`))