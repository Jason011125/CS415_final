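; BP_Magnet is a pickup that instantly collects nearby coins for the third-person pawn that touches its Sensor.
; On overlap it runs a sphere overlap around itself, ignoring the pawn and itself, and destroys any coins found.
; Each regular coin adds one to the pawn's Coin count, while gold coins add a larger bonus.
; It then plays a pull sound and destroys itself, with no physical attraction of the coins.
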(event `self.Sensor.OnComponentBeginOverlap`
  (params (OverlappedComponent :type "PrimitiveComponent Object Reference") (OtherActor :type "Actor Object Reference") (OtherComp :type "PrimitiveComponent Object Reference") (OtherBodyIndex :type Integer) (bFromSweep :type Boolean) (SweepResult :type "HitResult Structure (by ref)"))
  (bind _asbp_third_person_pawn (cast `/Game/VisualSandbox/Blueprints/GameModes/ThirdPerson/BP_ThirdPerson_Pawn` OtherActor))
  (bind _outactors (`KismetSystemLibrary.SphereOverlapActors` (`self.K2_GetActorLocation`) 1500.0 (`self.Object Types`) null (`|MakeArray` _asbp_third_person_pawn self :!type "Actor Object Reference")))
  (for _array_element _outactors
    (bind _asbp_coin (cast `/Game/VisualSandbox/Blueprints/Pickups/Drop_Out/BP_Coin` _array_element)
      (:`then`
        (set `/Game/VisualSandbox/Blueprints/GameModes/ThirdPerson/BP_ThirdPerson_Pawn.Coin` (+ (`/Game/VisualSandbox/Blueprints/GameModes/ThirdPerson/BP_ThirdPerson_Pawn.Coin` _asbp_third_person_pawn) 1) _asbp_third_person_pawn)
        (`self.K2_DestroyActor` _asbp_coin))
      (:`CastFailed`
        (bind _asbp_gold_coin (cast `/Game/VisualSandbox/Blueprints/Pickups/Drop_Out/BP_GoldCoin` _array_element))
        (set `/Game/VisualSandbox/Blueprints/GameModes/ThirdPerson/BP_ThirdPerson_Pawn.Coin` (+ (`/Game/VisualSandbox/Blueprints/GameModes/ThirdPerson/BP_ThirdPerson_Pawn.Coin` _asbp_third_person_pawn) 100) _asbp_third_person_pawn)
        (`self.K2_DestroyActor` _asbp_gold_coin))))
  (`GameplayStatics.PlaySoundAtLocation` "/Engine/VREditor/Sounds/UI/Laser_Pull.Laser_Pull" (`self.K2_GetActorLocation`) (struct) 1.0 1.0 0.0 null null null null)
  (`self.K2_DestroyActor`))

(fn `UserConstructionScript`)