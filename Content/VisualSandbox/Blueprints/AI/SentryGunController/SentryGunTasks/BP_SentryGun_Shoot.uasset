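; Behavior tree task that makes a sentry gun fire a set number of shots.
; On execute it runs the parent logic, resets a DoN counter and binds to the gun pawn's shot-fired event.
; Each tick calls Shoot on the pawn, while the event advances the counter and finishes the task successfully once NumberOfShots is reached.
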(event `self.ReceiveExecuteAI`
  (params (OwnerController :type "AIController Object Reference") (ControlledPawn :type "Pawn Object Reference"))
  (`parent.ReceiveExecuteAI` OwnerController ControlledPawn)
  (`self.RestartCounter`)
  (add `/Game/VisualSandbox/Blueprints/Weapons/SentryGun/BP_SentryGun.On Shot Fired` (`self.SentryGunPawn`) (delegate `OnShotFired`)))

(event `OnShotFired`
  (bind _numberofshots (`self.NumberOfShots`))
  ;[1 1 1] Shots counter
  (bind _counter (`/Engine/EditorBlueprintResources/StandardMacros.Do N` _numberofshots :!label _label)
    (:`Exit`
      (if (>= _counter _numberofshots)
        (`self.FinishExecute` true)))))

(event `self.ReceiveTickAI`
  (params (OwnerController :type "AIController Object Reference") (ControlledPawn :type "Pawn Object Reference") (DeltaSeconds :type "Float (single-precision)"))
  (`/Game/VisualSandbox/Blueprints/Weapons/SentryGun/BP_SentryGun.Shoot` (`self.SentryGunPawn`)))

(event `RestartCounter`
  ;[1 1 1] Shots counter
  (goto _label :!via `Reset`))