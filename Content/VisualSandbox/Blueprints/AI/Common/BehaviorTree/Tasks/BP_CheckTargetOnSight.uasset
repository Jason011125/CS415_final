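; Behavior Tree task that waits until the AI has its blackboard Target directly in its line of sight.
; Each tick it line traces on the Camera channel from the controller's eye viewpoint along the view direction, ignoring the controlled pawn.
; It finishes with success when the blocking hit is the Target actor; it has no failure path, so it keeps running otherwise.
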(event `self.ReceiveTickAI`
  (params (OwnerController :type "AIController Object Reference") (ControlledPawn :type "Pawn Object Reference") (DeltaSeconds :type "Float (single-precision)"))
  (bind (_outlocation _outrotation) (`Actor.GetActorEyesViewPoint` OwnerController))
  (bind _outhit (`KismetSystemLibrary.LineTraceSingle` _outlocation (+ _outlocation (* (`KismetMathLibrary.GetForwardVector` _outrotation) 100000.0)) "TraceTypeQuery2" false (`|MakeArray` ControlledPawn :!type "Actor Object Reference")))
  (bind (_bblockinghit _binitialoverlap _time _distance _location _impactpoint _normal _impactnormal _physmat _hitactor) (`GameplayStatics.BreakHitResult` _outhit))
  (if _bblockinghit
    (if (== _hitactor (`BTFunctionLibrary.GetBlackboardValueAsActor` (`self.Target`)))
      (`self.FinishExecute` true))))