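; AI controller for bots that runs a behavior tree and feeds it enemy, noise and damage information through the Blackboard.
; Perception updates record sighted enemies as threats, heard noise locations and a damage flag, dropping threats on failed sensing.
; Each tick it keeps threats that are alive and on another team, then sets the nearest as the enemy.
; A helper smoothly interpolates control rotation toward a target.
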(event `self.ReceiveBeginPlay`
  (bind _btasset (`self.BTAsset`)
    (:`then`
      (`self.RunBehaviorTree` _btasset))
    (:`else`)))

(event `self.AIPerception.OnTargetPerceptionUpdated`
  (params (Actor :type "Actor Object Reference") (Stimulus :type "AIStimulus Structure"))
  (`self.Update Perception` Actor Stimulus))

(event `self.ReceiveTick`
  (params (DeltaSeconds :type "Float (single-precision)"))
  (`self.Choose Enemy`))

(fn `Choose Enemy`
  (locals (I :type "Actor Object Reference") (BestThreats :type "Array of Actor Object Reference"))
  (if (`KismetArrayLibrary.Array_IsEmpty` (`self.ThreatsFound`))
    (`self.Set Enemy` null)
    (else
      (for _array_element (`self.ThreatsFound`) :!pinned true
        ;[1 1 1] LoopBody to find valid threats and add to "Best Targets" array
        (bind _output_get (set `local.I` _array_element))
        (`/Engine/EditorBlueprintResources/StandardMacros.IsValid` _output_get
          (:`Is Valid`
            (if (`self.Is Enemy` _output_get)
              (`KismetArrayLibrary.Array_AddUnique` (`local.BestThreats`) (`local.I`))))))
      ;[1 1 1] Checks if the "Best Taget" array is empty
      (bind _output_get_2 (set `self.ThreatsFound` (`local.BestThreats`)))
      (if (`KismetArrayLibrary.Array_IsEmpty` _output_get_2)
        (`self.Set Enemy` null)
        (else
          ;[1 1 1] Select the nearest actor as best enemy target
          (`self.Set Enemy` (`/Game/VisualSandbox/Blueprints/Utility/BP_UsefulFunctions.Find Nearest Actor` (`self.ThreatsFound`) (`self.K2_GetPawn`))))))))

(fn `Filter Enemy`
  (params (Actors :type "Array of Actor Object Reference"))
  (returns (`Return Enemies` :type "Array of Actor Object Reference"))
  (locals (a :type "Actor Object Reference") (`Enemy Found` :type "Array of Actor Object Reference"))
  (for _array_element Actors
    (bind _output_get (set `local.a` _array_element))
    (if (`self.Is Enemy` _output_get)
      (`KismetArrayLibrary.Array_Add` (`local.Enemy Found`) (`local.a`))))
  (return (`local.Enemy Found`)))

(fn `Is Enemy`
  (params (Target :type "Actor Object Reference"))
  (returns (ReturnValue :type Boolean))
  (locals (`Target Is Alive` :type Boolean :default false) (`Target Team Index` :type Integer :default 0) (`Pawn Team Index` :type Integer :default 0))
  (`|ExecutionSequence`
    (:`then_0`
      (bind _returnvalue (message `/Game/VisualSandbox/Blueprints/Interfaces/BPI_Bot.Is Alive` (`local.Target`)))
      (set `local.Target Is Alive` _returnvalue)
      (bind _returnvalue_2 (message `/Game/VisualSandbox/Blueprints/Interfaces/BPI_Bot.Get Team Index` (`local.Target`)))
      (set `local.Target Team Index` _returnvalue_2)
      (bind _returnvalue_3 (message `/Game/VisualSandbox/Blueprints/Interfaces/BPI_Bot.Get Team Index` (`self.K2_GetPawn`)))
      (set `local.Pawn Team Index` _returnvalue_3))
    (:`then_1`
      (return (and (`local.Target Is Alive`) (> (`local.Target Team Index`) -1) (!= (`local.Target Team Index`) (`local.Pawn Team Index`)))))))

(fn `Set Bot Control Rotation`
  (params (`New Control Rotation` :type "Rotator Structure") (`Control Rotation Lag` :type "Float (double-precision)"))
  (returns (Successful :type Boolean))
  (`self.SetControlRotation` (`KismetMathLibrary.RInterpTo` (`self.GetControlRotation`) (`local.New Control Rotation`) (`GameplayStatics.GetWorldDeltaSeconds`) (`local.Control Rotation Lag`)))
  (return (== (`self.GetControlRotation`) (`local.New Control Rotation`) :`ErrorTolerance` 10.0)))

(fn `Set Enemy`
  (params (NewTarget :type "Actor Object Reference"))
  (`BlackboardComponent.SetValueAsObject` (`self.Blackboard`) (`self.EnemyKey`) (`local.NewTarget`)))

(fn `Update Perception`
  (params (Actor :type "Actor Object Reference") (Stimulus :type "AIStimulus Structure"))
  (bind (_stimulus_age _stimulus_expirationage _stimulus_strength _stimulus_stimuluslocation _stimulus_receiverlocation _stimulus_tag _stimulus_bsuccessfullysensed) (break `AIStimulus` (`local.Stimulus`)))
  (bind (_stimulus_age_2 _stimulus_expirationage_2 _stimulus_strength_2 _stimulus_stimuluslocation_2) (break `AIStimulus` (`local.Stimulus`)))
  (`|ExecutionSequence`
    (:`then_0`
      (if _stimulus_bsuccessfullysensed
        (`|ExecutionSequence`
          (:`then_0`
            ; Sight Sense
            (bind _returnvalue (`AIPerceptionSystem.GetSenseClassForStimulus` (`local.Stimulus`)))
            (if (== _returnvalue "/Script/AIModule.AISense_Sight")
              (if (`self.Is Enemy` (`local.Actor`))
                (`KismetArrayLibrary.Array_AddUnique` (`self.ThreatsFound`) (`local.Actor`)))))
          (:`then_1`
            ; Nosie Sense
            (bind _returnvalue_2 (`AIPerceptionSystem.GetSenseClassForStimulus` (`local.Stimulus`)))
            (if (== _returnvalue_2 "/Script/AIModule.AISense_Hearing")
              (if (!= (`local.Actor`) (`self.K2_GetPawn`))
                (`BlackboardComponent.SetValueAsVector` (`self.Blackboard`) (`self.Noise Location Key`) _stimulus_stimuluslocation_2))))
          (:`then_2`
            ; Sense damage
            (bind _returnvalue_3 (`AIPerceptionSystem.GetSenseClassForStimulus` (`local.Stimulus`)))
            (if (== _returnvalue_3 "/Script/AIModule.AISense_Damage")
              (`BlackboardComponent.SetValueAsBool` (`self.Blackboard`) (`self.Taking Damage Key`) true))))
        (else
          (`KismetArrayLibrary.Array_RemoveItem` (`self.ThreatsFound`) (`local.Actor`)))))
    (:`then_1`
      (`BlackboardComponent.SetValueAsBool` (`self.Blackboard`) (`self.Enemy Spotted Key`) (not (`KismetArrayLibrary.Array_IsEmpty` (`self.ThreatsFound`)))))))

(fn `UserConstructionScript`)