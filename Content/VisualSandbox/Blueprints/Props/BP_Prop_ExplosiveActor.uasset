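; BP_Prop_ExplosiveActor is a prop that explodes, optionally when it takes any damage.
; Explode is guarded against repeats; on authority it records the instigator, disables further damage, sets a short lifespan and spawns an explosion using the configured type, ignored actors and radial force.
; Outside the authority check, it also stops mesh physics, disables collision and hides the actor wherever Explode runs.
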(event `self.ReceiveAnyDamage`
  (params (Damage :type "Float (single-precision)") (DamageType :type "DamageType Object Reference") (InstigatedBy :type "Controller Object Reference") (DamageCauser :type "Actor Object Reference"))
  ; Explode when take damage
  (if (`self.Can Explode On Take Damage`)
    (`self.Explode` InstigatedBy)))

(fn `Explode`
  (params (`Explosion Instigator` :type "Controller Object Reference"))
  (if (not (`self.Is Exploding`))
    (`|ExecutionSequence`
      (:`then_0`
        (`/Engine/EditorBlueprintResources/ActorMacros.Switch Has Authority`
          (:`Authority`
            (set `self.Explosion Instigator` (`local.Explosion Instigator`))
            (set `self.bCanBeDamaged` false)
            (`self.SetLifeSpan` 1.0)
            (`/Game/VisualSandbox/Blueprints/Utility/BP_UsefulFunctions.Spawn Explosion` (`self.K2_GetActorLocation`) (`self.Explosion Type`) (`self.Actors To Ignore`) self (`self.Explosion Instigator`) (`self.RadialForce`))
            (set `self.Is Exploding` true))))
      (:`then_1`
        (`PrimitiveComponent.SetSimulatePhysics` (`self.StaticMeshComponent`) false)
        (`self.SetActorEnableCollision` false)
        (`self.SetActorHiddenInGame` true)))))

(fn `UserConstructionScript`)