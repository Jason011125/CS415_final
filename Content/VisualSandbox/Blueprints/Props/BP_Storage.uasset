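; BP_Storage is a storage prop, such as a chest, that holds items in a StorageInventory.
; When an item is added, it is hidden and attached to the prop at a named socket, keeping its world scale.
; Its inventory getter returns the InventoryServer's inventory when that reference is valid, otherwise its own.
; The health system getter returns nothing and UseItem always returns false.
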(event `self.Storage Inventory.On Items Added`
  (params (Item :type "/Game/VisualSandbox/Blueprints/Pickups/Items/BP_Item Object Reference"))
  ; Attach the new added item to chest and disable visibility
  (`self.SetActorHiddenInGame` Item true)
  (`self.K2_AttachToActor` Item self (`self.Attach Socket Name`) "SnapToTarget" "SnapToTarget" "KeepWorld" true))

(fn `Get Health System`
  (returns (`Health Conp` :type "/Game/VisualSandbox/Blueprints/Components/AC_HealthComponent Object Reference"))
  (return null))

(fn `Get Inventory System`
  (returns (`Inventory Comp` :type "/Game/VisualSandbox/Blueprints/Components/AC_InventoryComponent Object Reference"))
  (bind _inventory_server (`self.Inventory Server`)
    (:`then`
      (return (`/Game/VisualSandbox/Blueprints/Systems/BP_Inventory_Network.Inventory` _inventory_server)))
    (:`else`
      (return (`self.Storage Inventory`)))))

(fn `Use Item`
  (params (`Item To Use` :type "/Game/VisualSandbox/Blueprints/Pickups/Items/BP_Item Object Reference"))
  (returns (Successful :type Boolean))
  (return false))

(fn `UserConstructionScript`)