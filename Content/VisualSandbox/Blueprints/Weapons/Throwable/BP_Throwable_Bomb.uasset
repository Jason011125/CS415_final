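; Throwable bomb item that explodes on a detonation timer or as soon as it takes damage.
; Pulling the pin, automatic at BeginPlay when AutoExplode is set, plays a sound, starts the timer, blocks pickup and activates the trail.
; Explode clears the timer, spawns the configured explosion and hides the mesh, while the authority disables damage and sets a short lifespan.
; Fast impacts play a bouncing sound.
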(event `self.ReceiveBeginPlay`
  ; Pulls the pin at the beginning of the game
  (`parent.ReceiveBeginPlay`)
  (if (`self.Auto Explode`)
    (`self.Pull The Pin`)))

(event `self.ReceiveHit`
  (params (MyComp :type "PrimitiveComponent Object Reference") (Other :type "Actor Object Reference") (OtherComp :type "PrimitiveComponent Object Reference") (bSelfMoved :type Boolean) (HitLocation :type "Vector Structure") (HitNormal :type "Vector Structure") (NormalImpulse :type "Vector Structure") (Hit :type "HitResult Structure (by ref)"))
  ; Play bouncing sound on hit
  (`self.Play Bouncing` HitLocation))

(event `self.ReceiveAnyDamage`
  (params (Damage :type "Float (single-precision)") (DamageType :type "DamageType Object Reference") (InstigatedBy :type "Controller Object Reference") (DamageCauser :type "Actor Object Reference"))
  ; Explode when take damage
  (if (> Damage 0.0)
    (`self.Explode`)))

(fn `Explode`
  (bind _item_mesh (`self.Item Mesh`))
  (`KismetSystemLibrary.K2_ClearAndInvalidateTimerHandle` (`self.Detonation Timer`))
  (`|ExecutionSequence`
    (:`then_0`
      (`/Engine/EditorBlueprintResources/ActorMacros.Switch Has Authority`
        (:`Authority`
          (set `self.bCanBeDamaged` false)
          (`self.SetLifeSpan` 1.0))))
    (:`then_1`
      (`/Game/VisualSandbox/Blueprints/Utility/BP_UsefulFunctions.Spawn Explosion` (`self.K2_GetActorLocation`) (`self.Explosion Type`) (`self.Actors To Ignore`) self (`self.GetInstigatorController`) (`self.Explosion Force`))
      (`self.SetActorEnableCollision` false)
      (`PrimitiveComponent.SetSimulatePhysics` _item_mesh false)
      (`SceneComponent.SetVisibility` _item_mesh false false))))

(fn `Play Bouncing`
  (params (`Hit Location` :type "Vector Structure"))
  (locals (`Grenade Velocity` :type "Float (double-precision)" :default 0.0))
  (set `local.Grenade Velocity` (`KismetMathLibrary.VSize` (`self.GetVelocity`)))
  (if (> (`local.Grenade Velocity`) 250.0)
    (`GameplayStatics.PlaySoundAtLocation` (`self.Bouncing Sound`) (`local.Hit Location`) (struct) 1.0 1.0 0.0 null null null null)))

(fn `Pull The Pin`
  (if (not (`KismetSystemLibrary.K2_IsValidTimerHandle` (`self.Detonation Timer`)))
    (`GameplayStatics.PlaySoundAtLocation` (`self.Pin Sound`) (`self.K2_GetActorLocation`) (struct) 1.0 1.0 0.0 null null null null) ; Play pin sound
    (bind _returnvalue (`KismetSystemLibrary.K2_SetTimer` null "Explode" (`self.Detonation Time`))) ; set grenade detonation timer
    (set `self.Detonation Timer` _returnvalue)
    (set `self.Can Be Picked up` false) ; set can be picked up to false
    (`ActorComponent.Activate` (`self.Trail`) true)))

(fn `UserConstructionScript`
  (`parent.UserConstructionScript`))