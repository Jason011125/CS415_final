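; Rocket launcher firearm Blueprint that defines how the weapon levels up.
; LevelUp raises Level by one until MaxLevel and adds one to MaxRounds whenever the new level is odd.
; The construction script only calls its parent, and the event graph holds only disabled placeholder events, so this graph logic adds no firing behavior.
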(fn `LevelUp`
  (if (< (`self.Level`) (`self.MaxLevel`))
    (set `self.Level` (+ (`self.Level`) 1))
    (if (== (mod (`self.Level`) 2) 1)
      (set `self.Max Rounds` (+ (`self.Max Rounds`) 1)))))

(fn `UserConstructionScript`
  (`parent.UserConstructionScript`))