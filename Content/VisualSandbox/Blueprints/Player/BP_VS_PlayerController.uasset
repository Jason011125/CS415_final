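; Player controller for VisualSandbox that handles pausing, cursor visibility and input mapping contexts.
; It registers its Enhanced Input context on BeginPlay, with guarded add/remove events.
; The pause action toggles game pause, messages the HUD's pause menu, switches cursor and input mode, restores prior cursor visibility and toggles pawn input.
; Look applies sensitivity and optional vertical inversion but is gated by CanLook, which returns false here.
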(event `EnhancedInput|/Game/VisualSandbox/Blueprints/Inputs/Game/IA_Pause`
  (params (ActionValue :type Boolean) (ElapsedSeconds :type "Float (double-precision)") (TriggeredSeconds :type "Float (double-precision)") (InputAction :type "InputAction Object Reference" :default "/Game/VisualSandbox/Blueprints/Inputs/Game/IA_Pause.IA_Pause"))
  ; Pause the game
  (:`Started`
    (`/Game/VisualSandbox/Blueprints/Interfaces/BPI_Game.Set Pause Game` (not (`GameplayStatics.IsGamePaused`)))))

(event `self.ReceiveBeginPlay`
  ; Add Player Controller Input Mapping Context
  (`self.Add IMC Asset` (`self.Player Controller IMC Asset`)))

(event `/Game/VisualSandbox/Blueprints/Interfaces/BPI_Game.Add IMC Asset`
  (params (`IMC to Add` :type "InputMappingContext Object Reference") (Priority :type Integer))
  (bind _returnvalue (subsystem `EnhancedInputLocalPlayerSubsystem`))
  ; Add IMC Asset
  (if (not (`.ReturnValue` (`EnhancedInputSubsystemInterface.HasMappingContext` _returnvalue `IMC to Add`)))
    (`EnhancedInputSubsystemInterface.AddMappingContext` _returnvalue `IMC to Add` Priority (struct))))

(event `/Game/VisualSandbox/Blueprints/Interfaces/BPI_Game.Remove IMC Asset`
  (params (`IMC to Remove` :type "InputMappingContext Object Reference"))
  (bind _returnvalue (subsystem `EnhancedInputLocalPlayerSubsystem`))
  ; Remove IMC Asset
  (if (`.ReturnValue` (`EnhancedInputSubsystemInterface.HasMappingContext` _returnvalue `IMC to Remove`))
    (`EnhancedInputSubsystemInterface.RemoveMappingContext` _returnvalue `IMC to Remove` (struct))))

(fn `Can Look`
  (returns (ReturnValue :type Boolean))
  (return false))

(fn `Get Main Character`
  (returns (`Return Main Character` :type "Pawn Object Reference"))
  (return (`self.K2_GetPawn`)))

(fn `Look`
  (params (`Input Value` :type "Vector2D Structure"))
  (bind _returnvalue (`self.K2_GetPawn`))
  (bind (_returnvalue_x _returnvalue_y) (`KismetMathLibrary.BreakVector2D` (* (`local.Input Value`) (`self.Look Sensitivity`))))
  (if (`self.Can Look`)
    (`Pawn.AddControllerYawInput` _returnvalue _returnvalue_x)
    (`Pawn.AddControllerPitchInput` _returnvalue (`KismetMathLibrary.SelectFloat` _returnvalue_y (* _returnvalue_y -1.0) (`self.Invert Look Vertical Axis`)))))

(fn `Set Mouse Cursor Visibility`
  (params (Visible :type Boolean) (`Display Position` :type "Vector2D Structure"))
  (bind (_locationx _locationy) (`self.GetMousePosition`))
  (bind _display_position (`local.Display Position`))
  (bind (_returnvalue_x _returnvalue_y) (`KismetMathLibrary.BreakVector2D` (select `bool` (!= _display_position (0.0 0.0)) :`false` (`KismetMathLibrary.MakeVector2D` _locationx _locationy) :`true` _display_position)))
  (bind _output_get (set `self.bShowMouseCursor` Visible))
  (if _output_get
    ; Set input game mode and mouse position
    (`WidgetBlueprintLibrary.SetInputMode_GameAndUIEx` self null "DoNotLock" false)
    (`self.SetMouseLocation` (`KismetMathLibrary.FTrunc` _returnvalue_x) (`KismetMathLibrary.FTrunc` _returnvalue_y))
    (else
      (`WidgetBlueprintLibrary.SetInputMode_GameOnly` self))))

(fn `Set Pause Game`
  (params (Pause :type Boolean))
  (returns (`Return Paused` :type Boolean))
  (bind _returnvalue (`self.K2_GetPawn`))
  (if Pause
    (set `self.Mouse Cursor Is Visible` (`self.bShowMouseCursor`)))
  (`GameplayStatics.SetGamePaused` (`local.Pause`))
  ; Dsiplay pause menu widget
  (message `/Game/VisualSandbox/Blueprints/Interfaces/BPI_HUD.Set Pause Menu Visibility` (`self.GetHUD`) (select `bool` (`local.Pause`) :`false` "NewEnumerator1" :`true` "NewEnumerator0" :!type "/Game/VisualSandbox/Blueprints/Enumerations/EWidgetVisibility Enum"))
  (`self.Set Mouse Cursor Visibility` (select `bool` (`local.Pause`) :`false` (`self.Mouse Cursor Is Visible`) :`true` true) (0.0 0.0))
  (`|ExecutionSequence`
    (:`then_0`
      ; Disable and enable pawn input
      (if (`local.Pause`)
        (`self.DisableInput` _returnvalue null)
        (else
          (`self.EnableInput` _returnvalue null))))
    (:`then_1`
      (return (`local.Pause`)))))

(fn `UserConstructionScript`)