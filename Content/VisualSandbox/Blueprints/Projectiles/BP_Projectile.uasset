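; Replicated projectile base that damages what it hits, pushes physics bodies and spawns impact effects.
; A component hit sets RepImpact, whose RepNotify runs OnImpact to share the impact across the network.
; OnImpact applies point damage to non-owners, reports it to AI sense, adds a velocity-aligned impulse, spawns surface-specific sound, FX and decal, then disables collision.
; The authority controls lifespan, shortening it after impact.
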(event `self.ReceiveBeginPlay`
  ; Set projectile life time
  (`/Engine/EditorBlueprintResources/ActorMacros.Switch Has Authority`
    (:`Authority`
      (`self.SetLifeSpan` (`self.Projectile Life Time`)))))

(event `self.Projectile Collision.OnComponentHit`
  (params (HitComponent :type "PrimitiveComponent Object Reference") (OtherActor :type "Actor Object Reference") (OtherComp :type "PrimitiveComponent Object Reference") (NormalImpulse :type "Vector Structure") (Hit :type "HitResult Structure (by ref)"))
  ; On projectile impacts
  (set `self.RepImpact` Hit))

(fn `Apply Impact Damage`
  (locals (ImpactLoc :type "Vector Structure" :default (0.0 0.0 0.0)))
  (bind _returnvalue (`self.GetOwner`))
  (bind (_proj_impact_result_bblockinghit _proj_impact_result_binitialoverlap _proj_impact_result_time _proj_impact_result_distance _proj_impact_result_location _proj_impact_result_impactpoint _proj_impact_result_normal _proj_impact_result_impactnormal _proj_impact_result_physmat _proj_impact_result_hitactor) (`GameplayStatics.BreakHitResult` (`self.Proj Impact Result`)))
  (bind (_proj_impact_result_bblockinghit_2 _proj_impact_result_binitialoverlap_2 _proj_impact_result_time_2 _proj_impact_result_distance_2 _proj_impact_result_location_2 _proj_impact_result_impactpoint_2 _proj_impact_result_normal_2 _proj_impact_result_impactnormal_2 _proj_impact_result_physmat_2 _proj_impact_result_hitactor_2) (`GameplayStatics.BreakHitResult` (`self.Proj Impact Result`)))
  (bind _impactloc (`local.ImpactLoc`))
  ; Apply Damage
  (`/Engine/EditorBlueprintResources/StandardMacros.IsValid` _returnvalue
    (:`Is Valid`
      (if (!= _returnvalue _proj_impact_result_hitactor_2)
        (`GameplayStatics.ApplyPointDamage` _proj_impact_result_hitactor_2 (`self.Damage`) (`self.GetVelocity`) (`self.Proj Impact Result`) (`self.GetInstigatorController` (`self.GetOwner`)) self (`self.DmgType`))
        ; Report Damage event
        (set `local.ImpactLoc` _proj_impact_result_location)
        (`AISense_Damage.ReportDamageEvent` _proj_impact_result_hitactor (`self.GetOwner`) (`self.Damage`) _impactloc _impactloc "Shots")))))

(fn `Apply Impact Impulse`
  (locals (ImpactLocation :type "Vector Structure" :default (0.0 0.0 0.0)))
  (bind (_proj_impact_result_bblockinghit _proj_impact_result_binitialoverlap _proj_impact_result_time _proj_impact_result_distance _proj_impact_result_location _proj_impact_result_impactpoint _proj_impact_result_normal _proj_impact_result_impactnormal _proj_impact_result_physmat _proj_impact_result_hitactor _proj_impact_result_hitcomponent _proj_impact_result_hitbonename) (`GameplayStatics.BreakHitResult` (`self.Proj Impact Result`)))
  (set `local.ImpactLocation` _proj_impact_result_location)
  (`/Engine/EditorBlueprintResources/StandardMacros.IsValid` _proj_impact_result_hitcomponent
    (:`Is Valid`
      (if (`SceneComponent.IsSimulatingPhysics` _proj_impact_result_hitcomponent _proj_impact_result_hitbonename)
        (`PrimitiveComponent.AddImpulseAtLocation` _proj_impact_result_hitcomponent (`self.Get Impulse Force`) (`local.ImpactLocation`) _proj_impact_result_hitbonename)))))

(fn `Get Impact Effects`
  (params (Surface :type "PhysicalMaterial Object Reference"))
  (returns (ReturnValue :type "/Game/VisualSandbox/Blueprints/Structures/FImpactEffects Structure"))
  (bind (_value _returnvalue) (`BlueprintMapLibrary.Map_Find` (`self.ImpactEffect`) (`local.Surface`)))
  (return (select `bool` _returnvalue :`false` (`self.DefaultImpactEffect`) :`true` _value)))

(fn `Get Impulse Force`
  (returns (ReturnValue :type "Vector Structure"))
  (return (* (`KismetMathLibrary.Normal` (`MovementComponent.Velocity` (`self.ProjectileMovement`))) (`self.ImpulsePower`))))

(fn `On Impact`
  (params (`Impact Result` :type "HitResult Structure"))
  (set `self.Proj Impact Result` `Impact Result`)
  (`|ExecutionSequence`
    (:`then_0`
      (`/Engine/EditorBlueprintResources/ActorMacros.Switch Has Authority`
        (:`Authority`
          (`self.SetLifeSpan` 1.0))))
    (:`then_1`
      (`self.Apply Impact Damage`)
      (`self.Apply Impact Impulse`)
      (`self.Spawn ImpactFX`)
      (`self.SetActorEnableCollision` false))))

(fn `OnRep_RepImpact`
  (`self.On Impact` (`self.RepImpact`)))

(fn `Spawn ImpactFX`
  (locals (ImpactEffects :type "/Game/VisualSandbox/Blueprints/Structures/FImpactEffects Structure") (ImpactLocation :type "Vector Structure" :default (0.0 0.0 0.0)) (ImpactNormal :type "Vector Structure" :default (0.0 0.0 0.0)))
  (bind (_proj_impact_result_bblockinghit _proj_impact_result_binitialoverlap _proj_impact_result_time _proj_impact_result_distance _proj_impact_result_location _proj_impact_result_impactpoint _proj_impact_result_normal _proj_impact_result_impactnormal _proj_impact_result_physmat) (`GameplayStatics.BreakHitResult` (`self.Proj Impact Result`)))
  (bind (_impacteffects_impactsound _impacteffects_impactfx _impacteffects_impactdecal _impacteffects_decalsize) (break `/Game/VisualSandbox/Blueprints/Structures/FImpactEffects` (`local.ImpactEffects`)))
  (bind (_impacteffects_impactsound_2 _impacteffects_impactfx_2) (break `/Game/VisualSandbox/Blueprints/Structures/FImpactEffects` (`local.ImpactEffects`)))
  (bind _impacteffects_impactsound_3 (break `/Game/VisualSandbox/Blueprints/Structures/FImpactEffects` (`local.ImpactEffects`)))
  ; Get impact data
  (set `local.ImpactLocation` _proj_impact_result_location)
  (set `local.ImpactNormal` _proj_impact_result_normal)
  (set `local.ImpactEffects` (`self.Get Impact Effects` _proj_impact_result_physmat))
  (`|ExecutionSequence`
    (:`then_0`
      ; Play Impact sound
      (`GameplayStatics.PlaySoundAtLocation` _impacteffects_impactsound_3 (`local.ImpactLocation`) (struct) 1.0 1.0 0.0 null null null null))
    (:`then_1`
      ; Spawn impact effect
      (`NiagaraFunctionLibrary.SpawnSystemAtLocation` _impacteffects_impactfx_2 (`local.ImpactLocation`) (`KismetMathLibrary.MakeRotationFromAxes` (`local.ImpactNormal`)) (1.0 1.0 1.0) true true "AutoRelease"))
    (:`then_2`
      ; Spawn impact decal
      (bind _returnvalue (`GameplayStatics.SpawnDecalAtLocation` _impacteffects_impactdecal _impacteffects_decalsize (`local.ImpactLocation`) (`KismetMathLibrary.MakeRotationFromAxes` (* (`local.ImpactNormal`) -1.0)) 30.0))
      (`/Engine/EditorBlueprintResources/StandardMacros.IsValid` _returnvalue
        (:`Is Valid`
          (`DecalComponent.SetFadeScreenSize` _returnvalue 0.001))))))

(fn `UserConstructionScript`)