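; Utility function library with shared helpers for math, nearest-actor lookup, condition-list checks, hitscan and explosions.
; Hitscan line-traces forward from an origin and applies point damage on a blocking hit.
; SpawnExplosion applies authority-only radial damage from explosion type data, scaled by player pawn 0's ATK with a CRIT roll adding CDMG, whoever owns the explosion.
; It also plays sound and Niagara effects, reports AI noise and fires an optional radial impulse.
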(fn `Check Condition List`
  (params (`Condition List` :type "Array of /Game/VisualSandbox/Blueprints/Structures/FConditionList Structure"))
  (returns (ReturnValue :type Boolean) (`Fail Reason` :type String))
  (locals (Successful :type Boolean :default true) (`Fail Message` :type String))
  (for _array_element `Condition List`
    (if (not (break `/Game/VisualSandbox/Blueprints/Structures/FConditionList` _array_element))
      (set `local.Successful` false)
      (set `local.Fail Message` (`.FailReason_17_041AEFF547EBCFCB03DEB8B8A54A3902` (break `/Game/VisualSandbox/Blueprints/Structures/FConditionList` _array_element)))))
  (return (`local.Successful`) (`local.Fail Message`)))

(fn `Find Nearest Actor`
  (params (ActorsToCheck :type "Array of Actor Object Reference (by ref)") (OtherActor :type "Actor Object Reference"))
  (returns (ReturnValue :type "Actor Object Reference"))
  (return (`.ReturnValue` (`GameplayStatics.FindNearestActor` (`Actor.K2_GetActorLocation` (`local.OtherActor`)) (`local.ActorsToCheck`)))))

(fn `Get Forward Location`
  (params (Location :type "Vector Structure") (Direction :type "Rotator Structure") (Distance :type "Float (double-precision)"))
  (returns (`Return Location` :type "Vector Structure"))
  (return (+ Location (* (`KismetMathLibrary.GetForwardVector` Direction) (`local.Distance`)))))

(fn `Hitscan`
  (params (Origin :type "Vector Structure") (Direction :type "Rotator Structure") (`Hitscan Distance` :type "Float (double-precision)" :default 100000.0) (`Hitscan Damage` :type "Float (double-precision)" :default 25.0) (`Hitscan Collision Channel` :type "ETraceTypeQuery Enum" :default "TraceTypeQuery3") (`Actors To Ignore` :type "Array of Actor Object Reference") (`Debug Hitscan` :type "EDrawDebugTrace Enum" :default "None") (Instigator :type "Controller Object Reference") (Causer :type "Actor Object Reference") (`Damage Type` :type "DamageType Class Reference"))
  (returns (`Hitscan Info` :type "HitResult Structure"))
  (locals (`Hitscan HR` :type "HitResult Structure"))
  (bind _origin (`local.Origin`))
  ; Draw line trace
  (bind _outhit (`KismetSystemLibrary.LineTraceSingle` (`local.Instigator`) _origin (`self.Get Forward Location` _origin (`local.Direction`) (`local.Hitscan Distance`) (`local.Instigator`)) (`local.Hitscan Collision Channel`) false (`local.Actors To Ignore`) (`local.Debug Hitscan`)))
  (bind _output_get (set `local.Hitscan HR` _outhit))
  (if (`GameplayStatics.BreakHitResult` _output_get)
    ; Apply point damage
    (`GameplayStatics.ApplyPointDamage` (`.HitActor` (`GameplayStatics.BreakHitResult` _output_get)) (`local.Hitscan Damage`) (`local.Origin`) (`local.Hitscan HR`) (`local.Instigator`) (`local.Causer`) (`local.Damage Type`))
    (return (`local.Hitscan HR`))))

(fn `Invert Float`
  (params (`Float Value` :type "Float (single-precision)") (`Invert Condition` :type Boolean))
  (returns (`Return Value` :type "Float (single-precision)"))
  (bind _float_value (`local.Float Value`))
  (return (`KismetMathLibrary.SelectFloat` (* _float_value -1.0) _float_value (`local.Invert Condition`))))

(fn `Spawn Explosion`
  (params (`Explosion Origin` :type "Vector Structure") (`Explosion Type` :type "/Game/VisualSandbox/Blueprints/Structures/FExplosionData Structure") (`Actor To Ignore` :type "Array of Actor Object Reference") (`Explosion Owner` :type "Actor Object Reference") (`Explosion Instigator` :type "Controller Object Reference") (`Explosion Force` :type "RadialForceComponent Object Reference"))
  (bind _explosion_origin (`local.Explosion Origin`))
  (bind _explosion_owner (`local.Explosion Owner`))
  (bind _explosion_owner_2 (`local.Explosion Owner`))
  (bind _explosion_origin_2 (`local.Explosion Origin`))
  (bind (_explosion_type_explosionsound _explosion_type_explosionfx _explosion_type_explosiondamage _explosion_type_explosionmindamage _explosion_type_explosioninnerradius _explosion_type_explosionouterradius) (break `/Game/VisualSandbox/Blueprints/Structures/FExplosionData` (`local.Explosion Type`)))
  (bind _actor_to_ignore (`local.Actor To Ignore`))
  (bind _explosion_owner_3 (`local.Explosion Owner`))
  (bind (_explosion_type_explosionsound_2 _explosion_type_explosionfx_2 _explosion_type_explosiondamage_2 _explosion_type_explosionmindamage_2 _explosion_type_explosioninnerradius_2 _explosion_type_explosionouterradius_2 _explosion_type_damagefalloff _explosion_type_damagetypeclass _explosion_type_damagepreventionchannel _explosion_type_explosionnoiseloudness _explosion_type_explosionnoiserange _explosion_type_explosionnoisetag) (break `/Game/VisualSandbox/Blueprints/Structures/FExplosionData` (`local.Explosion Type`)))
  (bind (_explosionsound _explosionfx _explosiondamage _explosionmindamage _explosioninnerradius _explosionouterradius _damagefalloff _damagetypeclass _damagepreventionchannel) (break `/Game/VisualSandbox/Blueprints/Structures/FExplosionData` (`local.Explosion Type`)))
  (`|ExecutionSequence`
    (:`then_0`
      ; Apply explosion damage
      (`KismetArrayLibrary.Array_Add` (`local.Actor To Ignore`) (`local.Explosion Owner`))
      (if (`Actor.HasAuthority` (`local.Explosion Owner`))
        (bind _asbp_third_person_pawn (cast `/Game/VisualSandbox/Blueprints/GameModes/ThirdPerson/BP_ThirdPerson_Pawn` (`GameplayStatics.GetPlayerPawn` null)))
        (if (<= (`KismetMathLibrary.RandomFloatInRange` 0.0 100.0) (`/Game/VisualSandbox/Blueprints/GameModes/ThirdPerson/BP_ThirdPerson_Pawn.CRIT` _asbp_third_person_pawn))
          (bind _returnvalue (/ (`/Game/VisualSandbox/Blueprints/GameModes/ThirdPerson/BP_ThirdPerson_Pawn.ATK` _asbp_third_person_pawn) 100.0))
          (bind _returnvalue_2 (* _explosiondamage _returnvalue))
          (bind _returnvalue_3 (/ (`/Game/VisualSandbox/Blueprints/GameModes/ThirdPerson/BP_ThirdPerson_Pawn.CDMG` _asbp_third_person_pawn) 100.0))
          (bind _returnvalue_4 (* _explosionmindamage _returnvalue))
          (`GameplayStatics.ApplyRadialDamageWithFalloff` _explosion_owner_2 (* _returnvalue_2 _returnvalue_3) (* _returnvalue_4 _returnvalue_3) _explosion_origin _explosioninnerradius _explosionouterradius _damagefalloff _damagetypeclass _actor_to_ignore _explosion_owner (`local.Explosion Instigator`) _damagepreventionchannel)
          (else
            (`GameplayStatics.ApplyRadialDamageWithFalloff` _explosion_owner_2 _returnvalue_2 _returnvalue_4 _explosion_origin _explosioninnerradius _explosionouterradius _damagefalloff _damagetypeclass _actor_to_ignore _explosion_owner null _damagepreventionchannel)))))
    (:`then_1`
      ; Spawn explosion sound and visual effects
      (`GameplayStatics.PlaySoundAtLocation` _explosion_owner_3 _explosion_type_explosionsound_2 _explosion_origin_2 (struct) 1.0 1.0 0.0 null null _explosion_owner_3 null)
      (`NiagaraFunctionLibrary.SpawnSystemAtLocation` _explosion_owner_3 _explosion_type_explosionfx_2 _explosion_origin_2)
      (`AISense_Hearing.ReportNoiseEvent` _explosion_owner_3 _explosion_origin_2 1.0 _explosion_owner_3 0.0 _explosion_type_explosionnoisetag)
      ; Apply explosion impulse
      (bind _explosion_force (`local.Explosion Force`)
        (:`then`
          (set `RadialForceComponent.Radius` _explosion_type_explosionouterradius _explosion_force)
          (`RadialForceComponent.FireImpulse` _explosion_force))
        (:`else`)))))

(fn `Spread Rotation`
  (params (Rotation :type "Rotator Structure") (SpreadAmount :type "Rotator Structure"))
  (returns (ReturnValue :type "Rotator Structure"))
  (bind _spreadamount (`local.SpreadAmount`))
  (bind (_returnvalue_roll _returnvalue_pitch _returnvalue_yaw) (`KismetMathLibrary.BreakRotator` (* _spreadamount -1.0)))
  (return (`KismetMathLibrary.MakeRotator` (+ (.roll Rotation) (`KismetMathLibrary.RandomFloatInRange` _returnvalue_roll (.roll _spreadamount))) (+ (.pitch Rotation) (`KismetMathLibrary.RandomFloatInRange` _returnvalue_pitch (.pitch _spreadamount))) (+ (.yaw Rotation) (`KismetMathLibrary.RandomFloatInRange` _returnvalue_yaw (.yaw _spreadamount))))))