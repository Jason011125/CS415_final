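; BP_Boss is a boss character with health, a Beholder attack animation and an on-screen health bar.
; BeginPlay creates the health widget, and Tick sets its bar from Health on a fixed scale of 100.
; AnyDamage subtracts from Health, then at zero disables movement and ragdolls the mesh.
; The Attack event plays a montage, using IsAttacking to block re-entry until it completes.
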(event `self.ReceiveAnyDamage`
  (params (Damage :type "Float (single-precision)") (DamageType :type "DamageType Object Reference") (InstigatedBy :type "Controller Object Reference") (DamageCauser :type "Actor Object Reference"))
  (set `self.Health` (- (`self.Health`) Damage))
  (if (<= (`self.Health`) 0.0)
    (`CharacterMovementComponent.DisableMovement` (`self.CharacterMovement`))
    (`PrimitiveComponent.SetSimulatePhysics` (`self.Mesh`) true)))

(event `self.ReceiveBeginPlay`
  (bind _returnvalue (`|CreateWidget` "/Game/VisualSandbox/Blueprints/Boss/WB_Boss_Health.WB_Boss_Health_C"))
  (`UserWidget.AddToViewport` _returnvalue 0)
  (set `self.HealthUI` _returnvalue))

(event `self.ReceiveTick`
  (params (DeltaSeconds :type "Float (single-precision)"))
  (`ProgressBar.SetPercent` (`/Game/VisualSandbox/Blueprints/Boss/WB_Boss_Health.Health_Bar` (`self.HealthUI`)) (/ (`self.Health`) 100.0)))

(event `/Game/VisualSandbox/Blueprints/Boss/BPI_BossFight.Attack`
  ; Attack
  (if (not (`self.IsAttacking?`))
    (`|PlayMontage` (`self.Mesh`) "/Game/MonsterForSurvivalGame/Animation/PBR/Beholder/Beholder_Attack01_ANIM_Montage.Beholder_Attack01_ANIM_Montage"
      (:`then`
        (set `self.IsAttacking?` true))
      (:`OnCompleted`
        (set `self.IsAttacking?` false)))))

(fn `UserConstructionScript`)