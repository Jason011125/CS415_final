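; BP_Mortar is an enemy that lobs BP_MortarShell projectiles at the player.
; PlayAttack solves a ballistic toss from Arrow1 to just beside the player's position with SuggestProjectileVelocity, then spawns a shell with that velocity if a solution exists.
; AnyDamage reduces Health and briefly raises IsHit; at zero Health, Die clears the state flags, disables movement and destroys the actor immediately.
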(event `self.ReceiveAnyDamage`
  (params (Damage :type "Float (single-precision)") (DamageType :type "DamageType Object Reference") (InstigatedBy :type "Controller Object Reference") (DamageCauser :type "Actor Object Reference"))
  (if (not (`self.bIsDead`))
    (bind _output_get (set `self.Health` (`KismetMathLibrary.FMax` (- (`self.Health`) Damage))))
    (set `self.bIsHit` true)
    (if (<= _output_get 0.0)
      (set `self.bIsDead` true)
      (`self.Die`)
      (else
        (`KismetSystemLibrary.Delay` 0.5)
        (set `self.bIsHit` false)))))

(event `Die`
  (set `self.bIsHit` false)
  (set `self.bIsAttacking` false)
  (`CharacterMovementComponent.DisableMovement` (`self.CharacterMovement`))
  (`self.K2_DestroyActor`))

(event `PlayAttack`
  (bind _arrow1 (`self.Arrow1`))
  (bind _returnvalue (`SceneComponent.K2_GetComponentLocation` _arrow1))
  (bind (_tossvelocity _returnvalue_2) (`GameplayStatics.BlueprintSuggestProjectileVelocity` _returnvalue (+ (`self.K2_GetActorLocation` (`GameplayStatics.GetPlayerPawn` 0)) (0.0 50.0 0.0)) 2000.0 0.0 "DoNotTrace"))
  (if _returnvalue_2
    (bind _returnvalue_3 (`|SpawnActorFromClass` "/Game/MonsterForSurvivalGame/EnemyBlueprints/BP_MortarShell.BP_MortarShell_C" (`KismetMathLibrary.MakeTransform` _returnvalue (`SceneComponent.K2_GetComponentRotation` _arrow1)) "Undefined" "MultiplyWithRoot" self null))
    (set `MovementComponent.Velocity` _tossvelocity (`/Game/MonsterForSurvivalGame/EnemyBlueprints/BP_MortarShell.ProjectileMovement` _returnvalue_3))))

(fn `UserConstructionScript`)