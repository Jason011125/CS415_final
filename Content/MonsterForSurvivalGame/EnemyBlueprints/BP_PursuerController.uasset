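; AI controller for BP_Pursuer, an enemy that roams around its spawn point until it spots the player, then chases and attacks.
; Roaming re-issues a random reachable move one second after each request, without waiting for arrival.
; Pawn sensing triggers an AIMoveTo chase; reaching the player clears the seen flag and resumes roaming.
; While the player is seen, Tick triggers cooldown-limited attacks at close range.
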(event `StartRoaming`
  (if (not (`self.bHasSeenPlayer`))
    (`|AIMoveTo` (`self.K2_GetPawn`) (`NavigationSystemV1.K2_GetRandomReachablePointInRadius` (`self.Home location`) (`self.RoamRadius`) null null) null 100.0
      (:`then`
        (`KismetSystemLibrary.Delay` 1.0)
        (`self.StartRoaming`)))))

(event `self.ReceiveBeginPlay`
  (set `self.Home location` (`self.K2_GetActorLocation` (`self.K2_GetPawn`)))
  (`self.StartRoaming`))

(event `TryAttack`
  (bind _asbp_pursuer (cast `/Game/MonsterForSurvivalGame/EnemyBlueprints/BP_Pursuer` (`self.K2_GetPawn`)))
  (`/Game/MonsterForSurvivalGame/EnemyBlueprints/BP_Pursuer.PlayAttack` _asbp_pursuer))

(event `self.ReceiveTick`
  (params (DeltaSeconds :type "Float (single-precision)"))
  (if (`self.bHasSeenPlayer`)
    (if (and (<= (`KismetMathLibrary.Vector_Distance` (`self.K2_GetActorLocation` (`self.TargetActor`)) (`self.K2_GetActorLocation` (`self.K2_GetPawn`))) 200.0) (> (- (`KismetSystemLibrary.GetGameTimeInSeconds`) (`self.LastAttackTime`)) (`self.AttackCooldown`)))
      (set `self.LastAttackTime` (`KismetSystemLibrary.GetGameTimeInSeconds`))
      (`self.TryAttack`))))

(event `self.PawnSensing.OnSeePawn`
  (params (Pawn :type "Pawn Object Reference"))
  (if (not (`self.bHasSeenPlayer`))
    (set `self.bHasSeenPlayer` true)
    (set `self.TargetActor` (`GameplayStatics.GetPlayerCharacter` 0))
    (`self.StartChasingPlayer`)))

(event `StartChasingPlayer`
  (`|AIMoveTo` (`self.K2_GetPawn`) (0.0 0.0 0.0) (`self.TargetActor`) 75.0 true
    (:`OnSuccess`
      (set `self.bHasSeenPlayer` false)
      (`self.StartRoaming`))))

(fn `UserConstructionScript`)