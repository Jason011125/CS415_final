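; BP_Pursuer is a survival-game enemy that handles taking damage, dying and attacking the player.
; AnyDamage lowers Health and raises IsHit for a half-second reaction window, or sets IsDead and calls Die at zero.
; Die clears the state flags, disables movement and destroys the actor immediately.
; PlayAttack applies fixed damage to the first player character with no range check in this graph, plus a debug print.
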(event `self.ReceiveAnyDamage`
  (params (Damage :type "Float (single-precision)") (DamageType :type "DamageType Object Reference") (InstigatedBy :type "Controller Object Reference") (DamageCauser :type "Actor Object Reference"))
  (if (not (`self.bIsDead`))
    (bind _output_get (set `self.Health` (`KismetMathLibrary.FMax` (- (`self.Health`) Damage))))
    (set `self.bIsHit` true)
    (if (<= _output_get 0.0)
      (set `self.bIsDead` true)
      (`self.Die`)
      (else
        (`KismetSystemLibrary.Delay` 0.5)
        (set `self.bIsHit` false)))))

(event `Die`
  (set `self.bIsHit` false)
  (set `self.bIsAttacking` false)
  (`CharacterMovementComponent.DisableMovement` (`self.CharacterMovement`))
  (`self.K2_DestroyActor`))

(event `PlayAttack`
  (`GameplayStatics.ApplyDamage` (`GameplayStatics.GetPlayerCharacter` 0) 20.0)
  (`KismetSystemLibrary.PrintString` "attempt to deal damage"))

(fn `UserConstructionScript`)